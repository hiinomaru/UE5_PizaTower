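; Moon actor whose Sphere orbits the actor's pivot, driven by a referenced DirectionalLight.
; The construction script moves the actor to Center and sets the Sphere's relative location to Center plus OrbitDiameter on Y.
; Each Tick adds the light's full rotation to the actor's world rotation, so it accumulates per frame without delta-time scaling rather than matching the light.
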(event EventBeginPlay)

(event Collision|EventActorBeginOverlap
  (params (OtherActor :type Actor%20Object%20Reference)))

(event EventTick
  (params (DeltaSeconds :type Float%20%28single-precision%29))
  (Class|Actor|AddActorWorldRotation (Transformation|GetActorRotation (Variables|Default|GetDirectionalLight))))

(fn ConstructionScript
  (Transformation|SetActorLocation (Variables|Default|Getcenter) false false)
  (Transformation|SetRelativeLocation (Variables|Default|GetSphere) (+ (Variables|Default|Getcenter) (Math|Vector|MakeVector 0.0 (Variables|Default|GetOrbitDiameter) 0.0)) false false))